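; HeavyVirusBP is a virus enemy that moves along a Direction vector at a set speed and shows its health on a widget bar.
; On spawn it makes every Turret retarget, then after a fixed delay clears their targets, retargets them and destroys itself.
; ModifyHealth applies clamped damage, and zero health also destroys it.
; Any destruction plays a death sound and increments VirusHandler's counter, opening LosingScreen at the maximum.
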(event `self.ReceiveDestroyed`
  (`GameplayStatics.PlaySoundAtLocation` "/Game/Assets/Sounds/VirusDeathSE.VirusDeathSE")
  (bind _outactors (`GameplayStatics.GetAllActorsOfClass` "/Game/Assets/Blueprints/VirusHandler.VirusHandler_C"))
  (bind _output (`|GetArrayItem` _outactors))
  (bind _result (`/Engine/EditorBlueprintResources/StandardMacros.IncrementInt` (`/Game/Assets/Blueprints/VirusHandler.VirusCounter` _output))
    (:`  `
      (if (>= _result (`/Game/Assets/Blueprints/VirusHandler.MaxVirus` _output))
        (`GameplayStatics.OpenLevel` "LosingScreen")))))

(event `self.ReceiveBeginPlay`
  (bind _outactors (`GameplayStatics.GetAllActorsOfClass` "/Game/Assets/Blueprints/Turret/Turret.Turret_C"))
  (for _array_element _outactors
    (`/Game/Assets/Blueprints/Turret/Turret.TargetVirus` _array_element))
  (`KismetSystemLibrary.Delay` 11.0)
  (bind _outactors_2 (`GameplayStatics.GetAllActorsOfClass` "/Game/Assets/Blueprints/Turret/Turret.Turret_C"))
  (for _array_element_2 _outactors_2
    (set `/Game/Assets/Blueprints/Turret/Turret.TargettedPolyVirus` null _array_element_2)
    (`/Game/Assets/Blueprints/Turret/Turret.TargetVirus` _array_element_2))
  (`self.K2_DestroyActor`))

(event `self.ReceiveTick`
  (params (DeltaSeconds :type "Float (single-precision)"))
  ;[1 1 1] Virus Movement
  ;;[1 1 1] Update Location Every Frame
  (bind _ashealth_bar (cast `/Game/Assets/Widgets/HealthBar` (`WidgetComponent.GetUserWidgetObject` (`self.Widget`))))
  (`ProgressBar.SetPercent` (`/Game/Assets/Widgets/HealthBar.ProgressBar_213` _ashealth_bar) (/ (`self.health`) 100.0))
  (`self.K2_SetActorTransform` (`KismetMathLibrary.MakeTransform` (+ (* (`KismetMathLibrary.Normal` (`self.Direction`)) (* (`self.Speed`) (`GameplayStatics.GetWorldDeltaSeconds`))) (.location (`self.GetTransform`))) (.rotation (`self.GetTransform`)) (.scale (`self.GetTransform`))))
  ;[1 1 1] Kill Virus
  (if (<= (`self.health`) 0.0)
    (`self.K2_DestroyActor`)))

(fn `modifyHealth`
  (params (healthToSubtract :type "Float (double-precision)"))
  (set `self.health` (`KismetMathLibrary.FClamp` (- (`self.health`) healthToSubtract) 0.0 (`self.maxHealth`))))

(fn `UserConstructionScript`)
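; VirusSpawnBP is a spawn location that opens a UI button for spawning an actor at its SpawnPoint.
; Its EnableSpawningUI event creates a SpawnButton widget for the first player, passes it the SpawnPoint world transform and adds it to the viewport.
; It then switches input to game and UI with a visible cursor, and stores the widget as the player controller's CurrentButton.
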(event `EnableSpawningUI`
  (bind _returnvalue (`GameplayStatics.GetPlayerController` 0))
  ;[1 1 1] Spawn Actor Through Widget
  (bind _returnvalue_2 (`|CreateWidget` "/Game/Assets/Widgets/SpawnButton.SpawnButton_C" (`GameplayStatics.GetPlayerController` 0)))
  (set `/Game/Assets/Widgets/SpawnButton.SpawnTransform` (`SceneComponent.K2_GetComponentToWorld` (`self.SpawnPoint`)) _returnvalue_2)
  (`UserWidget.AddToViewport` _returnvalue_2 0)
  (`WidgetBlueprintLibrary.SetInputMode_GameAndUIEx` _returnvalue _returnvalue_2 "DoNotLock" false)
  (set `PlayerController.bShowMouseCursor` true _returnvalue)
  (set `/Game/Assets/Blueprints/PlayerController.CurrentButton` _returnvalue_2 (cast `/Game/Assets/Blueprints/PlayerController` _returnvalue :!pure true)))

(fn `UserConstructionScript`)
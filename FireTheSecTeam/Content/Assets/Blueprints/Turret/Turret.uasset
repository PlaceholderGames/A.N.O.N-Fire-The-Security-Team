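; Turret Blueprint that turns toward VirusBP actors and fires while in range.
; Tick loops over all VirusBP actors, yaw-interpolating the Pews component toward each and refreshing Inrange, which only measures distance to the first one found.
; A self-recalling loop from BeginPlay spawns Barrel actors at socket Pew1 at the Firerate interval, or rechecks after a short retriggerable delay when out of range.
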(event `getplayerrange`
  ;[1 1 1] Player Range
  (bind _outactors (`GameplayStatics.GetAllActorsOfClass` "/Game/Assets/Blueprints/VirusBP.VirusBP_C"))
  (if (< (`self.GetDistanceTo` self (`|GetArrayItem` _outactors)) (`self.attackrange`))
    (set `self.inrange` true)
    (else
      (set `self.inrange` false))))

(event `self.ReceiveBeginPlay`
  (`self.Shootatplayer`))

(event `Shootatplayer`
  ;[1 1 1] Shoot at player
  (if (`self.inrange`)
    (`|SpawnActorFromClass` "/Game/Assets/Blueprints/Turret/barrel.barrel_C" (`SceneComponent.GetSocketTransform` (`self.Pews`) "Pew1" "RTS_World") "Undefined" "OverrideRootScale" null null)
    (`KismetSystemLibrary.RetriggerableDelay` (`self.firerate`))
    (`self.Shootatplayer`)
    (else
      (`KismetSystemLibrary.RetriggerableDelay` 0.5)
      (`self.Shootatplayer`))))

(event `TurretRotation`
  ;[1 1 1] Turret rotation
  (if (`self.inrange`)
    (`SceneComponent.K2_SetWorldRotation` (`self.Pews`) (`KismetMathLibrary.RInterpTo` (`SceneComponent.K2_GetComponentRotation` (`self.Pews`)) (`KismetMathLibrary.MakeRotator` 0.0 0.0 (.yaw (`KismetMathLibrary.FindLookAtRotation` (`SceneComponent.K2_GetComponentLocation` (`self.Pews`)) (`self.K2_GetActorLocation` (stale `self.ReceiveTick` _array_element))))) (`self.delta time`) (`self.rotation speed`)) false false)))

(event `self.ReceiveTick`
  (params (DeltaSeconds :type "Float (single-precision)"))
  ;[1 1 1] Turret rotation
  (bind _outactors (`GameplayStatics.GetAllActorsOfClass` "/Game/Assets/Blueprints/VirusBP.VirusBP_C"))
  (for _array_element _outactors
    (set `self.delta time` DeltaSeconds)
    (`self.TurretRotation`)
    (`self.getplayerrange`)))

(fn `UserConstructionScript`)
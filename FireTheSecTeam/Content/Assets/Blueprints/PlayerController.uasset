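; Player controller that handles left-click release on virus spawn tiles to show and dismiss their spawn button UI.
; Each release loops over all VirusSpawnBP actors, calling SpawnClick for every inactive one to enable the UI on the tile under the cursor.
; For an active one, a cursor hit on anything other than CurrentButton removes that button and clears every tile's active flag.
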(event `Key|LeftMouseButton`
  (params (Key :type "Key Structure"))
  (bind (_hitresult _returnvalue) (`self.GetHitResultUnderCursorByChannel` "TraceTypeQuery1"))
  (bind _currentbutton (`self.CurrentButton`))
  (:`Released`
    ;[1 1 1] Check if Button is Already Active
    (bind _outactors (`GameplayStatics.GetAllActorsOfClass` "/Game/Assets/Blueprints/VirusSpawnBP.VirusSpawnBP_C"))
    (for _array_element _outactors
      (if (`/Game/Assets/Blueprints/VirusSpawnBP.SpawningUI.IsActive` _array_element) :!label _label
        (if _returnvalue
          (if (not (== (`.HitActor` (`GameplayStatics.BreakHitResult` _hitresult)) _currentbutton))
            (`Widget.RemoveFromParent` _currentbutton)
            (set `self.CurrentButton` _currentbutton)
            (`KismetSystemLibrary.PrintText` "Button Disabled")
            (bind _outactors_2 (`GameplayStatics.GetAllActorsOfClass` "/Game/Assets/Blueprints/VirusSpawnBP.VirusSpawnBP_C"))
            (for _array_element_2 _outactors_2
              (set `/Game/Assets/Blueprints/VirusSpawnBP.SpawningUI.IsActive` false _array_element_2 :!label _label_2))
            (goto _label_2)))
        (else
          (`self.SpawnClick`))))
    (goto _label)))

(event `SpawnClick`
  ;[1 1 1] Trigger "Spawn" Button When Tile is Clicked
  (bind _asvirus_spawn_bp (cast `/Game/Assets/Blueprints/VirusSpawnBP` (`.HitActor` (`GameplayStatics.BreakHitResult` (`self.GetHitResultUnderCursorByChannel` "TraceTypeQuery1")))))
  (if (not (`/Game/Assets/Blueprints/VirusSpawnBP.SpawningUI.IsActive` _asvirus_spawn_bp))
    (`KismetSystemLibrary.PrintText` "Button Enabled")
    (`/Game/Assets/Blueprints/VirusSpawnBP.EnableSpawningUI` _asvirus_spawn_bp)
    (set `/Game/Assets/Blueprints/VirusSpawnBP.SpawningUI.IsActive` true _asvirus_spawn_bp)))

(fn `UserConstructionScript`)
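; Level goal trigger that counts actors breaching the firewall and opens the NextLevelMenu level once the count reaches WinningNumber.
; On BeginPlay it writes its NextLevelTrigger value into NextLevelMenu's NextLevel.
; Any overlap increments the count without filtering by class.
; Short of the win, every Turret clears its target and retargets, a breach sound plays at world origin per turret, then the overlapping actor is destroyed.
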(event `self.ReceiveBeginPlay`
  ;[1 1 1] Set Next Level
  (bind _asnext_level_menu (cast `/Game/Assets/Widgets/NextLevelMenu` (`self.NextLevelMenu`)))
  (set `/Game/Assets/Widgets/NextLevelMenu.NextLevel` (`self.NextLevelTrigger`) _asnext_level_menu))

(event `self.Trigger.OnComponentBeginOverlap`
  (params (OverlappedComponent :type "PrimitiveComponent Object Reference") (OtherActor :type "Actor Object Reference") (OtherComp :type "PrimitiveComponent Object Reference") (OtherBodyIndex :type Integer) (bFromSweep :type Boolean) (SweepResult :type "HitResult Structure (by ref)"))
  ;[1 1 1] Trigger Winning Box
  (bind _result (`/Engine/EditorBlueprintResources/StandardMacros.IncrementInt` (`self.behindFirewall`))
    (:`  `
      (set `self.behindFirewall` _result)
      (if (>= (`self.behindFirewall`) (`self.winningNumber`))
        (`GameplayStatics.OpenLevel` "NextLevelMenu")
        (else
          (bind _outactors (`GameplayStatics.GetAllActorsOfClass` "/Game/Assets/Blueprints/Turret/Turret.Turret_C"))
          (for _array_element _outactors
            (set `/Game/Assets/Blueprints/Turret/Turret.TargettedPolyVirus` null _array_element)
            (`/Game/Assets/Blueprints/Turret/Turret.TargetVirus` _array_element)
            (`GameplayStatics.PlaySoundAtLocation` "/Game/Assets/Sounds/FirewallBreach.FirewallBreach"))
          (`self.K2_DestroyActor` OtherActor))))))

(fn `UserConstructionScript`)
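; Medic virus unit in a turret-defense game that moves along a set direction and heals another Heavy (Trojan) or Medic virus.
; Box overlap latches a target; Tick then matches its speed and restores its health over time when the Y-distance check passes.
; Turrets are told to target viruses on spawn.
; Zero health destroys it, and destruction increments the VirusHandler counter, opening LosingScreen at the maximum.
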(event `self.ReceiveBeginPlay`
  (bind _outactors (`GameplayStatics.GetAllActorsOfClass` "/Game/Assets/Blueprints/Turret/Turret.Turret_C"))
  (for _array_element _outactors
    (`/Game/Assets/Blueprints/Turret/Turret.TargetVirus` _array_element)))

(event `self.ReceiveTick`
  (params (DeltaSeconds :type "Float (single-precision)"))
  (`self.HealthBarUpdate`)
  (`self.LocationUpdate`)
  (if (`self.Overlapped`)
    (if (`self.healingHeavy`)
      (`self.HealHeavy`)
      (elif (`self.healingMedic`)
        (`self.HealMedic`)))))

(event `LocationUpdate`
  ;[1 1 1] Update Location Every Frame
  (`self.K2_SetActorTransform` (`KismetMathLibrary.MakeTransform` (+ (* (`KismetMathLibrary.Normal` (`self.Direction_0`)) (* (`self.medicSpeed`) (`GameplayStatics.GetWorldDeltaSeconds`))) (.location (`self.GetTransform`))) (.rotation (`self.GetTransform`)) (.scale (`self.GetTransform`))))
  ;[1 1 1] Kill Virus
  (if (<= (`self.medicHealth`) 0.0)
    (`self.K2_DestroyActor`)))

(event `self.Box.OnComponentBeginOverlap`
  (params (OverlappedComponent :type "PrimitiveComponent Object Reference") (OtherActor :type "Actor Object Reference") (OtherComp :type "PrimitiveComponent Object Reference") (OtherBodyIndex :type Integer) (bFromSweep :type Boolean) (SweepResult :type "HitResult Structure (by ref)"))
  ;[1 1 1] Check what type of virus is being healed
  (bind _asheavy_virus_bp (cast `/Game/Assets/Blueprints/HeavyVirusBP` OtherActor)
    (:`then`
      (set `self.healingMedic` false)
      (set `self.healingHeavy` true))
    (:`CastFailed`
      (bind _asmedic_virus_bp (cast `/Game/Assets/Blueprints/MedicVirusBP` OtherActor))
      (set `self.healingMedic` true)
      (set `self.healingHeavy` false)))
  (if (or (and (== _asmedic_virus_bp OtherActor) (!= _asmedic_virus_bp self)) (== _asheavy_virus_bp OtherActor) (== OtherActor "/Game/Assets/Blueprints/VirusBP.VirusBP"))
    (if (not (`self.Overlapped`))
      (set `self.Overlapped` true)
      (set `self.healedVirus` OtherActor))))

(event `HealthBarUpdate`
  ;[1 1 1] Health Bar Update
  (bind _ashealth_bar (cast `/Game/Assets/Widgets/HealthBar` (`WidgetComponent.GetUserWidgetObject` (`self.Widget_0`))))
  (`ProgressBar.SetPercent` (`/Game/Assets/Widgets/HealthBar.ProgressBar_213` _ashealth_bar) (/ (`self.medicHealth`) (`self.medicMaxHealth`))))

(event `self.ReceiveDestroyed`
  ;[1 1 1] Update Virus Counter
  (`GameplayStatics.PlaySoundAtLocation` "/Game/Assets/Sounds/VirusDeathSE.VirusDeathSE")
  (bind _outactors (`GameplayStatics.GetAllActorsOfClass` "/Game/Assets/Blueprints/VirusHandler.VirusHandler_C"))
  (bind _output (`|GetArrayItem` _outactors))
  (bind _result (`/Engine/EditorBlueprintResources/StandardMacros.IncrementInt` (`/Game/Assets/Blueprints/VirusHandler.VirusCounter` _output))
    (:`  `
      (if (>= _result (`/Game/Assets/Blueprints/VirusHandler.MaxVirus` _output))
        (`GameplayStatics.OpenLevel` "LosingScreen")))))

(event `HealHeavy`
  ;[1 1 1] HealHeavy - Heales the Trojan Virus in fron of the medic
  (bind _asheavy_virus_bp (cast `/Game/Assets/Blueprints/HeavyVirusBP` (`self.healedVirus`)))
  (`/Engine/EditorBlueprintResources/StandardMacros.IsValid` _asheavy_virus_bp
    (:`Is Valid`
      (if (<= (.y (- (.location (`self.GetTransform` _asheavy_virus_bp)) (.location (`self.GetTransform`)))) (.y (`self.TriggerDistance`)))
        ;;[1 1 1] Change Medic Virus to Same Speed as Healed Virus
        (set `self.medicSpeed` (`/Game/Assets/Blueprints/HeavyVirusBP.trojanSpeed` _asheavy_virus_bp))
        (if (< (`/Game/Assets/Blueprints/HeavyVirusBP.trojanHealth` _asheavy_virus_bp) (`/Game/Assets/Blueprints/HeavyVirusBP.trojanMaxHealth` _asheavy_virus_bp))
          ;;[1 1 1] Reged Health Every Tick
          (set `/Game/Assets/Blueprints/HeavyVirusBP.trojanHealth` (+ (`/Game/Assets/Blueprints/HeavyVirusBP.trojanHealth` _asheavy_virus_bp) (* (`GameplayStatics.GetWorldDeltaSeconds`) (`self.healing`))) _asheavy_virus_bp)
          (`/Game/Assets/Blueprints/HeavyVirusBP.HealthBarUpdate` _asheavy_virus_bp))))
    (:`Is Not Valid`
      (set `self.medicSpeed` 100.0))))

(event `HealMedic`
  ;[1 1 1] HealMedic - Heales the ILOVEYOU Virus in fron of this one
  (bind _asmedic_virus_bp (cast `/Game/Assets/Blueprints/MedicVirusBP` (`self.healedVirus`)))
  (`/Engine/EditorBlueprintResources/StandardMacros.IsValid` _asmedic_virus_bp
    (:`Is Valid`
      (if (<= (.y (- (.location (`self.GetTransform` _asmedic_virus_bp)) (.location (`self.GetTransform`)))) (.y (`self.TriggerDistance`)))
        ;;[1 1 1] Change Medic Virus to Same Speed as Healed Virus
        (set `self.medicSpeed` (`/Game/Assets/Blueprints/MedicVirusBP.medicSpeed` _asmedic_virus_bp))
        (if (< (`/Game/Assets/Blueprints/MedicVirusBP.medicHealth` _asmedic_virus_bp) (`/Game/Assets/Blueprints/MedicVirusBP.medicMaxHealth` _asmedic_virus_bp))
          ;;[1 1 1] Reged Health Every Tick
          (set `/Game/Assets/Blueprints/MedicVirusBP.medicHealth` (+ (`/Game/Assets/Blueprints/MedicVirusBP.medicHealth` _asmedic_virus_bp) (* (`GameplayStatics.GetWorldDeltaSeconds`) (`self.healing`))) _asmedic_virus_bp)
          (`self.HealthBarUpdate` _asmedic_virus_bp))))
    (:`Is Not Valid`
      (set `self.medicSpeed` 100.0))))

(fn `modifyHealth`
  (params (healthToSubtract :type "Float (double-precision)"))
  (set `self.medicHealth` (`KismetMathLibrary.FClamp` (- (`self.medicHealth`) healthToSubtract) 0.0 (`self.medicMaxHealth`))))

(fn `UserConstructionScript`)